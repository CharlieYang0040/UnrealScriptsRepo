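; BP_CamFollowLight places a target light on the far side of a skeletal mesh character from a target camera, facing the camera.
; It runs only from the Construction Script, with no Tick update.
; The light starts at the Bip001-Spine2 bone plus an offset, then moves along the normalized camera-to-character direction, Z flipped, by CameraDistance.
; It then rotates toward the camera and applies local roll, pitch and yaw offsets.
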(event EventBeginPlay)

(event Collision|EventActorBeginOverlap
  (params (OtherActor :type Actor%20Object%20Reference)))

(event EventTick
  (params (DeltaSeconds :type Float%20%28single-precision%29)))

(fn ConstructionScript
  (CallFunction|FTCamFollowSet))

(fn FTCamFollowSet
  (bind _targetlight (Variables|target1|GetTargetLight))
  (bind _targetcamera (Variables|target1|GetTargetCamera))
  (bind _targetcharacter (Variables|target1|GetTargetCharacter))
  (bind _returnvalue (Transformation|GetActorLocation _targetcamera))
  (bind _as스켈레탈_메시_액터 (Utilities|Casting|CastToSkeletalMeshActor _targetcharacter))
  (bind _outposition (Class|SkinnedMeshComponent|TransformfromBoneSpace (Variables|/Script/Engine.SkeletalMeshActor|GetSkeletalMeshComponent _as스켈레탈_메시_액터) "Bip001-Spine2" "0, 0, 0" "0, 0, 0"))
  (Transformation|SetActorLocation _targetlight (+ (Variables|location1|GetLocation%20Offset) _outposition) false false)
  (Transformation|AddActorWorldOffset _targetlight (* (Math|Vector|Normalize (* (- (Transformation|GetActorLocation _targetcharacter) _returnvalue) "1.000000,1.000000,-1.000000")) (Variables|location1|GetCamera%20Distance)))
  (Transformation|SetActorRotation _targetlight (Math|Rotator|FindLookatRotation (Transformation|GetActorLocation _targetlight) _returnvalue))
  (Transformation|AddActorLocalRotation _targetlight (Math|Rotator|MakeRotator (Variables|rotation1|GetRot%20Roll%20Offset) (Variables|rotation1|GetRot%20Pitch%20Offset) (Variables|rotation1|GetRot%20Yaw%20Offset)) false false))