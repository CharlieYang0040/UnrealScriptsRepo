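; Post-process actor that applies an outline and rim light material with editable color, size, rim angle and depth distance settings.
; The construction script puts the material in the first blendable slot of its PostProcess, keeping that slot's weight.
; A helper reuses a dynamic instance or creates one from a Material or Material Instance, printing on cast failure.
; The parameters are written to that instance, which then replaces the slot's material.
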(event EventBeginPlay)

(event Collision|EventActorBeginOverlap
  (params (OtherActor :type Actor%20Object%20Reference)))

(event EventTick
  (params (DeltaSeconds :type Float%20%28single-precision%29)))

(fn ConstructionScript
  (CallFunction|FTPPControl (Variables|Default|GetPostProcess) (Variables|Default|GetPostProcessMaterial)))

(fn FTPPControl
  (params (PP :type Post%20Process%20Component%20Object%20Reference) (PPMI :type Object%20Object%20Reference))
  (bind _parametername (Variables|Default|GetParameterName))
  (bind _settings (Variables|/Script/Engine.PostProcessComponent|GetSettings PP))
  (bind _weightedblendables (Utilities|Struct|BreakPostProcessSettings _settings))
  (bind _returnvalue (Utilities|String|StringToName _parametername))
  (bind _array (Utilities|Struct|BreakWeightedBlendables _weightedblendables))
  (bind _output (Utilities|Array|Get(acopy) _array))
  (bind (_weight _object) (Utilities|Struct|BreakWeightedBlendable _output))
  (Utilities|Array|SetArrayElem _array 0 (Utilities|Struct|MakeWeightedBlendable _weight PPMI))
  (bind _dynamicoutput (CallFunction|FTCastDynamic _object))
  (bind _output_get (Variables|Local|SetDynamicMaterial _dynamicoutput))
  (Rendering|Material|SetVectorParameterValue _output_get _returnvalue (Math|Conversions|ToLinearColor(Color) (Variables|Default|GetParameterColor)) :!class /Script/Engine.MaterialInstanceDynamic)
  (Rendering|Material|SetScalarParameterValue _output_get _returnvalue (Variables|Default|GetParameterScalar) :!class /Script/Engine.MaterialInstanceDynamic)
  (Rendering|Material|SetVectorParameterValue _output_get "LineColor" (Math|Conversions|ToLinearColor(Color) (Variables|Parameter|GetLineColor)) :!class /Script/Engine.MaterialInstanceDynamic)
  (Rendering|Material|SetScalarParameterValue _output_get "OutlineColorV" (Variables|Parameter|GetOutlineColorV) :!class /Script/Engine.MaterialInstanceDynamic)
  (Rendering|Material|SetScalarParameterValue _output_get "OutlineSizeMax" (Variables|Parameter|GetOutlineSizeMax) :!class /Script/Engine.MaterialInstanceDynamic)
  (Rendering|Material|SetScalarParameterValue _output_get "LineColorMult" (Variables|Parameter|GetLineColorMult) :!class /Script/Engine.MaterialInstanceDynamic)
  (Rendering|Material|SetScalarParameterValue _output_get "RimAngle(Screen)" (Variables|Parameter|GetRimAngle%28Screen%29) :!class /Script/Engine.MaterialInstanceDynamic)
  (Rendering|Material|SetScalarParameterValue _output_get "RimAngleOffset" (Variables|Parameter|GetRimAngleOffset) :!class /Script/Engine.MaterialInstanceDynamic)
  (Rendering|Material|SetScalarParameterValue _output_get "RimAngleSmooth" (Variables|Parameter|GetRimAngleSmooth) :!class /Script/Engine.MaterialInstanceDynamic)
  (Rendering|Material|SetScalarParameterValue _output_get "DepthDistance" (Variables|Parameter|GetDepthDistance) :!class /Script/Engine.MaterialInstanceDynamic)
  (Utilities|Array|SetArrayElem _array 0 (Utilities|Struct|MakeWeightedBlendable _weight _output_get))
  (return))

(fn FTCastDynamic
  (params (ObjectInput :type Object%20Object%20Reference))
  (bind _as머티리얼_인스턴스_다이내믹 (Utilities|Casting|CastToMaterialInstanceDynamic ObjectInput)
    (:then
      (Development|PrintString (Utilities|GetDisplayName _as머티리얼_인스턴스_다이내믹) false false)
      (return _as머티리얼_인스턴스_다이내믹))
    (:CastFailed
      (bind _as머티리얼 (Utilities|Casting|CastToMaterial ObjectInput)
        (:then
          (bind _returnvalue (Rendering|Material|CreateDynamicMaterialInstance _as머티리얼 "None" "None" :!class /Script/Engine.KismetMaterialLibrary))
          (Development|PrintString (Utilities|GetDisplayName _returnvalue) false false)
          (return _returnvalue))
        (:CastFailed
          (bind _as머티리얼_인스턴스 (Utilities|Casting|CastToMaterialInstance ObjectInput)
            (:then
              (bind _returnvalue_2 (Rendering|Material|CreateDynamicMaterialInstance _as머티리얼_인스턴스 "None" "None" :!class /Script/Engine.KismetMaterialLibrary))
              (Development|PrintString (Utilities|GetDisplayName _returnvalue_2) false false)
              (return _returnvalue_2))
            (:CastFailed
              (Development|PrintString (Utilities|String|Append "Cast Failed! 
Object Name : " (Utilities|GetObjectName ObjectInput) " 
Display Name : " (Utilities|GetDisplayName ObjectInput))))))))))