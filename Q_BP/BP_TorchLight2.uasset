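; BP_TorchLight2 is a torch light controller that sets the intensity of the Light actors in its TorchLights array.
; The Construction Script casts each entry to Light and lerps between MinIntensity and MaxIntensity using a sine of Time times Speed, wrapped at 2π.
; The raw sine alpha can go negative, and Time is a variable that nothing here advances, as BeginPlay and Tick are empty.
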(event EventBeginPlay)

(event Collision|EventActorBeginOverlap
  (params (OtherActor :type Actor%20Object%20Reference)))

(event EventTick
  (params (DeltaSeconds :type Float%20%28single-precision%29)))

(fn ConstructionScript
  (bind _returnvalue (Math|Float|MultiplybyPi 2.0))
  (bind _time (Variables|Default|GetTime))
  (bind _minintensity (Variables|Default|GetMinIntensity))
  (bind _maxintensity (Variables|Default|GetMaxIntensity))
  (bind _speed (Variables|Default|GetSpeed))
  (bind _returnvalue_2 (* _time _speed))
  (bind _remainder (Math|Float|Division(WholeandRemainder) _returnvalue_2 _returnvalue))
  (bind _returnvalue_3 (Math|Trig|Sin(Radians) _remainder))
  (bind _returnvalue_4 (Math|Float|Lerp _minintensity _maxintensity _returnvalue_3))
  (for _array_element (Variables|Default|GetTorchLights)
    (bind _as라이트 (Utilities|Casting|CastToLight _array_element))
    (Development|PrintString (Utilities|String|ToString(Float) _returnvalue_4) false false)
    (Rendering|Components|Light|SetIntensity (Variables|/Script/Engine.Light|GetLightComponent _as라이트) _returnvalue_4)))