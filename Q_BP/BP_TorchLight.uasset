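; BP_TorchLight is a torch actor that flickers its point light, PointLightTorch00, by varying the intensity.
; FT_SinFlicker advances Time by TimeSpeed per call, then sums two sine waves, the secondary phase-shifted, with Perlin noise and an offset.
; The noise samples a random input rather than Time, giving uncorrelated jitter.
; The construction script resets Time; the event graph is empty, so nothing here calls the flicker.
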(event EventBeginPlay)

(event Collision|EventActorBeginOverlap
  (params (OtherActor :type Actor%20Object%20Reference)))

(event EventTick
  (params (DeltaSeconds :type Float%20%28single-precision%29)))

(fn ConstructionScript
  (Variables|SinFlicker|SetTime 0.0)
  (Development|PrintString "initialize torchlight" false false))

(fn FTSinFlicker
  (Development|PrintString "trigger activated!" false false)
  (bind _output_get (Variables|SinFlicker|SetTime (+ (Variables|SinFlicker|GetTime) (Variables|SinFlicker|GetTime_Speed))))
  (Development|PrintString (Utilities|String|ToString(Float) (+ (+ (+ (* (Variables|SinFlicker|GetAmplitude_Main) (Math|Trig|Sin(Radians) (* _output_get (Variables|SinFlicker|GetFrequency_Main)))) (* (Variables|SinFlicker|GetAmplitude_Secondary) (Math|Trig|Sin(Radians) (+ (* _output_get (Variables|SinFlicker|GetFrequency_Secondary)) (Variables|SinFlicker|GetPhase_Offset_Secondary))))) (* (Variables|SinFlicker|GetNoise_Strength) (Class|KismetMathLibrary|PerlinNoise1D (Math|Random|RandomFloatinRange -1.0 1.0)))) (Variables|SinFlicker|GetOffset))) false false)
  (Rendering|Components|Light|SetIntensity (Variables|Default|GetPointLight_torch00) (+ (+ (+ (* (Variables|SinFlicker|GetAmplitude_Main) (Math|Trig|Sin(Radians) (* _output_get (Variables|SinFlicker|GetFrequency_Main)))) (* (Variables|SinFlicker|GetAmplitude_Secondary) (Math|Trig|Sin(Radians) (+ (* _output_get (Variables|SinFlicker|GetFrequency_Secondary)) (Variables|SinFlicker|GetPhase_Offset_Secondary))))) (* (Variables|SinFlicker|GetNoise_Strength) (Class|KismetMathLibrary|PerlinNoise1D (Math|Random|RandomFloatinRange -1.0 1.0)))) (Variables|SinFlicker|GetOffset))))