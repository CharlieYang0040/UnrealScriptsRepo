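; BP_Sky_CN2 is a skydome actor that sets up a textured sky with wind flow and a sun disc.
; Its construction script creates a dynamic material instance on the dome mesh, offsets and yaws the dome, then passes sky texture, wind and horizon settings to the material.
; An optional directional light actor's forward vector orients the sun; without a valid one, sun opacity is set to zero.
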(fn ConstructionScript
  (bind _wind_direction (Variables|Movement|GetWind%20direction))
  (bind _skydome_mesh (Variables|Basic|GetSkydome_mesh))
  (bind (_x _y) (Math|Vector|BreakVector _wind_direction))
  ;[1 1 1] Assigning material to Sky SM
  (Rendering|Material|SetMaterial (Variables|Basic|GetSkydome_mesh) 0 (Variables|Default|GetSky_Material))
  (bind _returnvalue (Rendering|Material|CreateDynamicMaterialInstance (Variables|Basic|GetSkydome_mesh) 0 0 "None" :!class /Script/Engine.PrimitiveComponent))
  (Variables|Default|SetSky%20material _returnvalue)
  (Utilities|IsValid (Variables|Default|GetDirectional%20light%20actor)
    (:Is%20Valid
      ;[1 1 1] Rotating sun disc accordingly to directional light angle (if actor specified)
      (Rendering|Material|SetVectorParameterValue (Variables|Default|GetSky%20material) "Light direction" (Math|Conversions|ToLinearColor(Vector) (Math|Rotator|GetRotationXVector (Transformation|GetActorRotation (Variables|Default|GetDirectional%20light%20actor)))) :!class /Script/Engine.MaterialInstanceDynamic))
    (:Is%20Not%20Valid
      (Rendering|Material|SetScalarParameterValue (Variables|Default|GetSky%20material) "Sun Opacity" 0.0 :!class /Script/Engine.MaterialInstanceDynamic)))
  ;[1 1 1] Setting up skydome parameters
  (Transformation|AddRelativeLocation _skydome_mesh (Math|Vector|MakeVector 0.0 0.0 (Variables|Basic|GetSkydome%20offset)) false false)
  (Transformation|AddRelativeRotation _skydome_mesh (Math|Rotator|MakeRotator 0.0 0.0 (Variables|Basic|GetSkydome%20angle)) false false)
  ;[1 1 1] Setting up material parameters
  (Rendering|Material|SetTextureParameterValue (Variables|Default|GetSky%20material) "Sky Texture" (Variables|Basic|GetSky%20Texture))
  (Rendering|Material|SetVectorParameterValue (Variables|Default|GetSky%20material) "Wind direction" (Math|Conversions|ToLinearColor(Vector) (Math|Vector|MakeVector _x _y 0.0)) :!class /Script/Engine.MaterialInstanceDynamic)
  (Rendering|Material|SetScalarParameterValue (Variables|Default|GetSky%20material) "Wind speed" (Variables|Movement|GetWind%20speed) :!class /Script/Engine.MaterialInstanceDynamic)
  (Rendering|Material|SetScalarParameterValue (Variables|Default|GetSky%20material) "Wind flow distance" (Variables|Movement|GetWind%20flow%20distance) :!class /Script/Engine.MaterialInstanceDynamic)
  (Rendering|Material|SetScalarParameterValue (Variables|Default|GetSky%20material) "Wind flow faloff" (Variables|Movement|GetHorizon%20Height) :!class /Script/Engine.MaterialInstanceDynamic)
  (Rendering|Material|SetScalarParameterValue (Variables|Default|GetSky%20material) "Horizon factor" (Variables|Movement|GetHorizon%20speed) :!class /Script/Engine.MaterialInstanceDynamic))