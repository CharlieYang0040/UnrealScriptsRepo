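; BP_EmissiveFakeGI is a placeable emissive mesh actor, named as a fake global illumination source.
; The construction script builds a dynamic material instance from EmissiveMaterial, feeds it the exposed color and multiplier, and applies it to both sphere and plane meshes.
; SwitchSphere selects which of the two shapes is visible.
; All logic runs in the construction script, as the event graph holds only disabled default events.
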(event EventBeginPlay)

(event Collision|EventActorBeginOverlap
  (params (OtherActor :type Actor%20Object%20Reference)))

(event EventTick
  (params (DeltaSeconds :type Float%20%28single-precision%29)))

(fn ConstructionScript
  (bind _emissive_sphere (Variables|Default|GetEmissive_Sphere))
  (bind _emissive_plane (Variables|Default|GetEmissive_Plane))
  (bind _returnvalue (Rendering|Material|CreateDynamicMaterialInstance (Variables|General|GetEmissiveMaterial) "None" "None" :!class /Script/Engine.KismetMaterialLibrary))
  (Rendering|Material|SetScalarParameterValue _returnvalue "EmissiveMult" (Variables|Emmisive|GetEmissiveMult) :!class /Script/Engine.MaterialInstanceDynamic)
  (Rendering|Material|SetVectorParameterValue _returnvalue "EmissiveColor" (Math|Conversions|ToLinearColor(Color) (Variables|Emmisive|GetEmissiveColor)) :!class /Script/Engine.MaterialInstanceDynamic)
  (Rendering|Material|SetMaterial _emissive_sphere 0 _returnvalue)
  (Rendering|Material|SetMaterial _emissive_plane 0 _returnvalue)
  (if (Variables|일반|GetSwitch_Sphere)
    (Rendering|SetVisibility _emissive_sphere true false)
    (Rendering|SetVisibility _emissive_plane false false)
    (else
      (Rendering|SetVisibility _emissive_sphere false false)
      (Rendering|SetVisibility _emissive_plane true false))))