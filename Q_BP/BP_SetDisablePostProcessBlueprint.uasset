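; Utility actor that toggles the post-process Animation Blueprint on a hand-picked set of skeletal mesh actors in the level.
; Its Construction Script runs a function that loops over eleven fixed actor reference slots and skips invalid ones.
; Every SkeletalMeshComponent on each actor gets its DisablePostProcessBlueprint flag set from the actor's own variable.
; The event graph has no runtime logic.
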(event EventBeginPlay)

(event Collision|EventActorBeginOverlap
  (params (OtherActor :type Actor%20Object%20Reference)))

(event EventTick
  (params (DeltaSeconds :type Float%20%28single-precision%29)))

(fn ConstructionScript
  (CallFunction|FTSetDisablePostprocess))

(fn FTSetDisablePostprocess
  (for _array_element (Utilities|Array|MakeArray (Variables|Default|GetSkeletalMeshActor_1) (Variables|Default|GetSkeletalMeshActor_2) (Variables|Default|GetSkeletalMeshActor_3) (Variables|Default|GetSkeletalMeshActor_4) (Variables|Default|GetSkeletalMeshActor_5) (Variables|Default|GetSkeletalMeshActor_6) (Variables|Default|GetSkeletalMeshActor_7) (Variables|Default|GetSkeletalMeshActor_8) (Variables|Default|GetSkeletalMeshActor_9) (Variables|Default|GetSkeletalMeshActor_10) (Variables|Default|GetSkeletalMeshActor_11))
    (Utilities|IsValid _array_element
      (:Is%20Valid
        (for _array_element_2 (Actor|GetComponentsByClass _array_element "/Script/Engine.SkeletalMeshComponent")
          (Variables|/Script/Engine.SkeletalMeshComponent|SetbDisablePostProcessBlueprint _array_element_2 (Variables|Default|GetDisable%20Post%20Process%20Blueprint)))))))